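; BP_Motel1 is a modular motel building whose layout is assembled in the construction script from Level2 and Level3 flags.
; Level2 switches Rooms 1-6 to the ground-floor unit class, adds top-floor meshes and child-actor rooms at their locations, swaps side meshes and reveals stairs and trim.
; Level3, checked only within Level2, repeats this for Rooms 7-11 at a different yaw.
; The event graph holds no logic.
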(fn `UserConstructionScript`
  (if (`self.Level2`)
    ;[1 1 1] Change Rooms On GroundFloor
    (`ChildActorComponent.SetChildActorClass` (`self.Room1`) "/Game/Blueprints/Motel1/BP_Motel_Unit_1_LvL1_GroundFloor--.BP_Motel_Unit_1_LvL1_GroundFloor--_C")
    (`ChildActorComponent.SetChildActorClass` (`self.Room2`) "/Game/Blueprints/Motel1/BP_Motel_Unit_1_LvL1_GroundFloor--.BP_Motel_Unit_1_LvL1_GroundFloor--_C")
    (`ChildActorComponent.SetChildActorClass` (`self.Room3`) "/Game/Blueprints/Motel1/BP_Motel_Unit_1_LvL1_GroundFloor--.BP_Motel_Unit_1_LvL1_GroundFloor--_C")
    (`ChildActorComponent.SetChildActorClass` (`self.Room4`) "/Game/Blueprints/Motel1/BP_Motel_Unit_1_LvL1_GroundFloor--.BP_Motel_Unit_1_LvL1_GroundFloor--_C")
    (`ChildActorComponent.SetChildActorClass` (`self.Room5`) "/Game/Blueprints/Motel1/BP_Motel_Unit_1_LvL1_GroundFloor--.BP_Motel_Unit_1_LvL1_GroundFloor--_C")
    (`ChildActorComponent.SetChildActorClass` (`self.Room6`) "/Game/Blueprints/Motel1/BP_Motel_Unit_1_LvL1_GroundFloor--.BP_Motel_Unit_1_LvL1_GroundFloor--_C")
    ;[1 1 1] Add Top Floor
    (`AddComponent|NODE_AddStaticMeshComponent-0`)
    (`AddComponent|NODE_AddStaticMeshComponent-1`)
    (`AddComponent|NODE_AddChildActorComponent-0` :`RelativeTransform` (`KismetMathLibrary.MakeTransform` (`SceneComponent.RelativeLocation` (`self.Room1`)) (struct :`Yaw` -90.0)))
    (`AddComponent|NODE_AddChildActorComponent-1` :`RelativeTransform` (`KismetMathLibrary.MakeTransform` (`SceneComponent.RelativeLocation` (`self.Room2`)) (struct :`Yaw` -90.0)))
    (`AddComponent|NODE_AddChildActorComponent-2` :`RelativeTransform` (`KismetMathLibrary.MakeTransform` (`SceneComponent.RelativeLocation` (`self.Room3`)) (struct :`Yaw` -90.0)))
    (`AddComponent|NODE_AddChildActorComponent-3` :`RelativeTransform` (`KismetMathLibrary.MakeTransform` (`SceneComponent.RelativeLocation` (`self.Room4`)) (struct :`Yaw` -90.0)))
    (`AddComponent|NODE_AddChildActorComponent-4` :`RelativeTransform` (`KismetMathLibrary.MakeTransform` (`SceneComponent.RelativeLocation` (`self.Room5`)) (struct :`Yaw` -90.0)))
    (`AddComponent|NODE_AddChildActorComponent-5` :`RelativeTransform` (`KismetMathLibrary.MakeTransform` (`SceneComponent.RelativeLocation` (`self.Room6`)) (struct :`Yaw` -90.0)))
    ;[1 1 1] Change The ground Side
    (`StaticMeshComponent.SetStaticMesh` (`self.SM_Motel_Side1_Left_Ground`) "/Game/GrandRockMotel/Meshes/Motel_Blocks/Modified1/SM_Motel_Side2_Left_Ground--.SM_Motel_Side2_Left_Ground--")
    (`StaticMeshComponent.SetStaticMesh` (`self.SM_Motel_Side2_Right_Ground--`) "/Game/GrandRockMotel/Meshes/Motel_Blocks/Modified1/SM_Motel_Side2_Right_Ground--.SM_Motel_Side2_Right_Ground--")
    ;[1 1 1] Show top StoneParts
    (`SceneComponent.SetVisibility` (`self.InstancedStaticMesh1`) true false)
    (`SceneComponent.SetVisibility` (`self.Box_F600C9CD1`) true false)
    (`SceneComponent.SetVisibility` (`self.Box_F600C9CD`) true false)
    (`SceneComponent.SetVisibility` (`self.SM_Motel1_Stairs1_Left--`) true false)
    (`SceneComponent.SetVisibility` (`self.SM_Motel1_Stairs1_Right--`) true false)
    (if (`self.Level3`)
      ;[1 1 1] Adding New Rooms On SecondFloor
      (`ChildActorComponent.SetChildActorClass` (`self.Room8`) "/Game/Blueprints/Motel1/BP_Motel_Unit_1_LvL1_GroundFloor--.BP_Motel_Unit_1_LvL1_GroundFloor--_C")
      (`ChildActorComponent.SetChildActorClass` (`self.Room9`) "/Game/Blueprints/Motel1/BP_Motel_Unit_1_LvL1_GroundFloor--.BP_Motel_Unit_1_LvL1_GroundFloor--_C")
      (`ChildActorComponent.SetChildActorClass` (`self.Room10`) "/Game/Blueprints/Motel1/BP_Motel_Unit_1_LvL1_GroundFloor--.BP_Motel_Unit_1_LvL1_GroundFloor--_C")
      (`ChildActorComponent.SetChildActorClass` (`self.Room11`) "/Game/Blueprints/Motel1/BP_Motel_Unit_1_LvL1_GroundFloor--.BP_Motel_Unit_1_LvL1_GroundFloor--_C")
      (`ChildActorComponent.SetChildActorClass` (`self.Room7`) "/Game/Blueprints/Motel1/BP_Motel_Unit_1_LvL1_GroundFloor--.BP_Motel_Unit_1_LvL1_GroundFloor--_C")
      (`AddComponent|NODE_AddStaticMeshComponent-4`)
      (`AddComponent|NODE_AddStaticMeshComponent-5`)
      (`AddComponent|NODE_AddChildActorComponent-12` :`RelativeTransform` (`KismetMathLibrary.MakeTransform` (`SceneComponent.RelativeLocation` (`self.Room8`)) (struct :`Yaw` 180.0)))
      (`AddComponent|NODE_AddChildActorComponent-13` :`RelativeTransform` (`KismetMathLibrary.MakeTransform` (`SceneComponent.RelativeLocation` (`self.Room9`)) (struct :`Yaw` 180.0)))
      (`AddComponent|NODE_AddChildActorComponent-14` :`RelativeTransform` (`KismetMathLibrary.MakeTransform` (`SceneComponent.RelativeLocation` (`self.Room10`)) (struct :`Yaw` 180.0)))
      (`AddComponent|NODE_AddChildActorComponent-15` :`RelativeTransform` (`KismetMathLibrary.MakeTransform` (`SceneComponent.RelativeLocation` (`self.Room11`)) (struct :`Yaw` 180.0)))
      (`AddComponent|NODE_AddChildActorComponent-18` :`RelativeTransform` (`KismetMathLibrary.MakeTransform` (`SceneComponent.RelativeLocation` (`self.Room7`)) (struct :`Yaw` 180.0)))
      (`StaticMeshComponent.SetStaticMesh` (`self.SM_Motel_Side1_Left_Ground1`) "/Game/GrandRockMotel/Meshes/Motel_Blocks/Modified1/SM_Motel_Side2_Left_Ground--.SM_Motel_Side2_Left_Ground--")
      (`StaticMeshComponent.SetStaticMesh` (`self.SM_Motel_Side2_Right_Ground--1`) "/Game/GrandRockMotel/Meshes/Motel_Blocks/Modified1/SM_Motel_Side2_Right_Ground--.SM_Motel_Side2_Right_Ground--")
      (`SceneComponent.SetVisibility` (`self.SM_Motel1_Stairs1_Right--1`) true false)
      (`SceneComponent.SetVisibility` (`self.SM_Motel1_Stairs1_Left--1`) true false)
      (`SceneComponent.SetVisibility` (`self.InstancedStaticMesh3`) true false)
      (`SceneComponent.SetVisibility` (`self.Box_F600C9CD2`) true false)
      (`SceneComponent.SetVisibility` (`self.Box_F600C9CD3`) true false))))