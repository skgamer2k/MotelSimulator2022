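; Spline-driven power line actor that places poles and hangs cables between them, built entirely in the construction script.
; A first loop spawns a BP_PowerPole child actor at each spline point, aligned to the spline, with an index text label above it.
; A second loop attaches each pole's two cables to the next pole's connectors, sizing them by distance plus random slack and zeroing the last pole's cable lengths.
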(fn `UserConstructionScript`
  (bind _index_of_loop (`self.Index of Loop`))
  (bind _spline (`self.Spline`))
  (bind _returnvalue (`SplineComponent.GetRotationAtSplinePoint` _spline _index_of_loop "Local"))
  (bind _output (`|GetArrayItem` (`self.AllChildActorsOfPowerline`) (`self.IndexLoop2`)))
  (bind _output_2 (`|GetArrayItem` (`self.AllChildActorsOfPowerline`) (`self.Number of SplinePoints`)))
  (bind _returnvalue_2 (`KismetMathLibrary.Conv_VectorToTransform` (`SplineComponent.GetLocationAtSplinePoint` _spline _index_of_loop "Local")))
  (bind _output_3 (`|GetArrayItem` (`self.AllChildActorsOfPowerline`) (+ (`self.IndexLoop2`) 1)))
  (bind _cable0 (`/Game/Blueprints/Splines/BP_PowerPole.Cable0` _output))
  (bind _cable1 (`/Game/Blueprints/Splines/BP_PowerPole.Cable1` _output))
  (bind _con_0 (`/Game/Blueprints/Splines/BP_PowerPole.Con 0` _output_3))
  (bind _con_1 (`/Game/Blueprints/Splines/BP_PowerPole.Con 1` _output_3))
  (bind _output_get (set `self.Number of SplinePoints` (- (`SplineComponent.GetNumberOfSplinePoints` (`self.Spline`)) 0)))
  (for _index (range (+ _output_get 1))
    (set `self.Index of Loop` _index)
    (bind _returnvalue_3 (`AddComponent|NODE_AddChildActorComponent-0` :`RelativeTransform` _returnvalue_2))
    (`ChildActorComponent.SetChildActorClass` _returnvalue_3 "/Game/Blueprints/Splines/BP_PowerPole.BP_PowerPole_C")
    (bind _asbp_power_pole (cast `/Game/Blueprints/Splines/BP_PowerPole` (`ChildActorComponent.ChildActor` _returnvalue_3)))
    (`KismetArrayLibrary.Array_Add` (`self.AllChildActorsOfPowerline`) _asbp_power_pole)
    (`SceneComponent.K2_SetRelativeRotation` _returnvalue_3 _returnvalue false false)
    (bind _returnvalue_4 (`AddComponent|NODE_AddTextRenderComponent-0` :`RelativeTransform` (`KismetMathLibrary.MakeTransform` (`KismetMathLibrary.MakeVector` (.x (.location _returnvalue_2)) (.y (.location _returnvalue_2)) (+ (.z (.location _returnvalue_2)) 1200.0)) _returnvalue)))
    (`TextRenderComponent.K2_SetText` _returnvalue_4 (`KismetTextLibrary.Conv_IntToText` (`self.Index of Loop`))))
  (for _index_2 (range (+ (`self.Number of SplinePoints`) 1))
    (set `self.IndexLoop2` _index_2)
    (`|ExecutionSequence`
      (:`then_0`
        (`SceneComponent.K2_AttachToComponent` _cable0 _con_0 "None" "SnapToTarget" "SnapToTarget" "KeepWorld" true)
        (set `CableComponent.CableLength` (+ (`KismetMathLibrary.RandomFloatInRange` 0.0 20.0) (`KismetMathLibrary.VSize` (- (`SceneComponent.K2_GetComponentLocation` (`/Game/Blueprints/Splines/BP_PowerPole.Con 0` _output)) (`SceneComponent.K2_GetComponentLocation` _con_0)))) _cable0)
        (set `CableComponent.CableLength` 0.0 (`/Game/Blueprints/Splines/BP_PowerPole.Cable0` _output_2)))
      (:`then_1`
        (`SceneComponent.K2_AttachToComponent` _cable1 _con_1 "None" "SnapToTarget" "SnapToTarget" "KeepWorld" true)
        (set `CableComponent.CableLength` (+ (`KismetMathLibrary.RandomFloatInRange` 0.0 20.0) (`KismetMathLibrary.VSize` (- (`SceneComponent.K2_GetComponentLocation` (`/Game/Blueprints/Splines/BP_PowerPole.Con 1` _output)) (`SceneComponent.K2_GetComponentLocation` _con_1)))) _cable1)
        (set `CableComponent.CableLength` 0.0 (`/Game/Blueprints/Splines/BP_PowerPole.Cable1` _output_2))))))