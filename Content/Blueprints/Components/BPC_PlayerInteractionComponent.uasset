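; Player interaction component that highlights interactable objects in view and lets the player pick up and drop physics objects.
; A looping timer is set on BeginPlay, and CheckInteractable line-traces from the camera for BPI_Interactable actors, toggling custom depth on the hit component.
; Interact queries the target and, for physics pickups, grabs it with the supplied physics handle, or releases a carried one.
; Tick holds the carried object ahead of the camera at its original rotation.
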(event `Initialize Component`
  (params (`Physics Handle Reference` :type "PhysicsHandleComponent Object Reference"))
  (set `self.GrabberRef` `Physics Handle Reference`))

(event `self.ReceiveBeginPlay`
  (bind _returnvalue (`KismetSystemLibrary.K2_SetTimerDelegate` (`|CreateDelegate` :!event `CheckInteractable`) 0.1 true))
  (set `self.TraceTimerHandle` _returnvalue))

(event `CheckInteractable`
  (bind _returnvalue (`GameplayStatics.GetPlayerCameraManager` 0))
  (bind _hit_component (`self.Hit Component`))
  (bind _returnvalue_2 (`Actor.K2_GetActorLocation` _returnvalue))
  (if (not (`self.IsCarryingItem?`))
    (`KismetSystemLibrary.PrintString` "Hello")
    (bind _outhit (`KismetSystemLibrary.LineTraceSingle` :`Start` _returnvalue_2 :`End` (+ _returnvalue_2 (* (`KismetMathLibrary.GetForwardVector` (`Actor.K2_GetActorRotation` _returnvalue)) (`self.InteractionRange`))) :`TraceChannel` "TraceTypeQuery1" :`DrawDebugType` (`self.TraceDebug`)))
    (bind (_bblockinghit _binitialoverlap _time _distance _location _impactpoint _normal _impactnormal _physmat _hitactor _hitcomponent) (`GameplayStatics.BreakHitResult` _outhit))
    (if _bblockinghit
      (if (`KismetSystemLibrary.DoesImplementInterface` _hitactor "/Game/Blueprints/Interfaces/BPI_Interactable.BPI_Interactable_C")
        (set `self.Hit Actor` _hitactor)
        (bind _output_get (set `self.Hit Component` _hitcomponent))
        (`PrimitiveComponent.SetRenderCustomDepth` _output_get true))
      (else
        (`/Engine/EditorBlueprintResources/StandardMacros.IsValid` _hit_component
          (:`Is Valid`
            (`PrimitiveComponent.SetRenderCustomDepth` _hit_component false)
            (set `self.Hit Component` null)
            (set `self.Hit Actor` null)))))))

(event `Interact`
  (bind _hit_component (`self.Hit Component`))
  (bind _hit_actor (`self.Hit Actor`))
  (bind _returnvalue (`SceneComponent.K2_GetComponentRotation` _hit_component))
  (if (not (`self.IsCarryingItem?`))
    (`/Engine/EditorBlueprintResources/StandardMacros.IsValid` _hit_actor
      (:`Is Valid`
        (bind _interaction_type (message `/Game/Blueprints/Interfaces/BPI_Interactable.Interact` _hit_actor))
        (switch `/Game/Blueprints/Enums/E_InteractionType` _interaction_type
          (:`NewEnumerator1`
            (bind _distance_from_camera (message `/Game/Blueprints/Interfaces/BPI_Interactable.AttachToPhysicsHandle` _hit_actor))
            (set `self.Distance from Camera` _distance_from_camera)
            (`PhysicsHandleComponent.GrabComponentAtLocationWithRotation` (`self.GrabberRef`) _hit_component "None" (`SceneComponent.K2_GetComponentLocation` _hit_component) _returnvalue)
            (set `self.ComponentRotation` _returnvalue)
            (set `self.IsCarryingItem?` true)))))
    (else
      (`PhysicsHandleComponent.ReleaseComponent` (`self.GrabberRef`))
      (set `self.IsCarryingItem?` false))))

(event `self.ReceiveTick`
  (params (DeltaSeconds :type "Float (single-precision)"))
  (bind _returnvalue (`GameplayStatics.GetPlayerCameraManager` 0))
  (if (`self.IsCarryingItem?`)
    (`PhysicsHandleComponent.SetTargetLocationAndRotation` (`self.GrabberRef`) (+ (`Actor.K2_GetActorLocation` _returnvalue) (* (`KismetMathLibrary.GetForwardVector` (`Actor.K2_GetActorRotation` _returnvalue)) (`self.Distance from Camera`))) (`self.ComponentRotation`))))