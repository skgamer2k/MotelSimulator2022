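; BP_MasterItem is the master item actor, configured from a data table row to act as an inventory item, physics pickup or interactable.
; The construction script assigns static or skeletal meshes; BeginPlay caches item details and sounds, simulating physics only for physics pickups.
; Hard static mesh hits play a drop sound, throttled by the sound's duration.
; Interact plays the pickup sound and returns item type; AttachToPhysicsHandle returns camera distance.
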(event `self.ReceiveBeginPlay`
  (bind (_datatable _rowname) (break `DataTableRowHandle` (`self.ItemInfo`)))
  (bind (_datatable_2 _rowname_2) (break `DataTableRowHandle` (`self.ItemInfo`)))
  (`|ExecutionSequence`
    (:`then_0`
      (bind _returnvalue (`|GetDataTableRow` _datatable_2 _rowname_2)
        (:`then`
          (bind (_name _description _staticmesh _skeletalmesh _itemtype) (break `/Game/Blueprints/Structs/S_ItemInfo` _returnvalue))
          (`PrimitiveComponent.SetSimulatePhysics` (`self.Mesh_Static`) (select `/Game/Blueprints/Enums/E_InteractionType` _itemtype :`NewEnumerator1` true))
          (`PrimitiveComponent.SetCollisionProfileName` (`self.Mesh_Skeletal`) "PhysicsActor" true)
          (`PrimitiveComponent.SetSimulatePhysics` (`self.Mesh_Skeletal`) (select `/Game/Blueprints/Enums/E_InteractionType` _itemtype :`NewEnumerator1` true))
          (`KismetSystemLibrary.PrintString` "Ball"))))
    (:`then_1`
      (bind _returnvalue_2 (`|GetDataTableRow` _datatable _rowname)
        (:`then`
          (bind (_name_2 _description_2 _staticmesh_2 _skeletalmesh_2 _itemtype_2 _icon _sounds) (break `/Game/Blueprints/Structs/S_ItemInfo` _returnvalue_2))
          (set `self.Name` _name_2)
          (set `self.Description` _description_2)
          (set `self.Item Type` _itemtype_2)
          (set `self.Icon` _icon)
          (set `self.Sounds` _sounds))))))

(event `self.Mesh_Static.OnComponentHit`
  (params (HitComponent :type "PrimitiveComponent Object Reference") (OtherActor :type "Actor Object Reference") (OtherComp :type "PrimitiveComponent Object Reference") (NormalImpulse :type "Vector Structure") (Hit :type "HitResult Structure (by ref)"))
  (bind (_pickupsound _dropsound) (break `/Game/Blueprints/Structs/S_Sounds` (`self.Sounds`)))
  (if (> (`KismetMathLibrary.VSize` (`SceneComponent.GetComponentVelocity` (`self.Mesh_Static`))) 500.0)
    (`/Engine/EditorBlueprintResources/StandardMacros.DoOnce` false :!label _label
      (:`Completed`
        (`GameplayStatics.PlaySoundAtLocation` _dropsound (`SceneComponent.K2_GetComponentLocation` (`self.Mesh_Static`)) (struct) 1.0 1.0 0.0 null null null)
        (`KismetSystemLibrary.Delay` (`SoundBase.Duration` _dropsound))
        (goto _label :!via `Reset`)))))

(fn `AttachToPhysicsHandle`
  (returns (`Distance From Camera` :type "Float (double-precision)"))
  (return (`self.Distance from Camera`)))

(fn `Interact`
  (returns (`Interaction Type` :type "/Game/Blueprints/Enums/E_InteractionType Enum"))
  (`GameplayStatics.PlaySoundAtLocation` (`.PickupSound_5_69954D2C4C533BFAF6C0BCB07B95D059` (break `/Game/Blueprints/Structs/S_Sounds` (`self.Sounds`))) (`self.K2_GetActorLocation`) (struct) 1.0 1.0 0.0 null null null)
  (return (`self.Item Type`)))

(fn `UserConstructionScript`
  (bind (_datatable _rowname) (break `DataTableRowHandle` (`self.ItemInfo`)))
  (bind _returnvalue (`|GetDataTableRow` _datatable _rowname)
    (:`then`
      (bind (_name _description _staticmesh _skeletalmesh) (break `/Game/Blueprints/Structs/S_ItemInfo` _returnvalue))
      (`/Engine/EditorBlueprintResources/StandardMacros.IsValid` _staticmesh
        (:`Is Valid`
          (`StaticMeshComponent.SetStaticMesh` (`self.Mesh_Static`) _staticmesh))
        (:`Is Not Valid`
          _))
      (`/Engine/EditorBlueprintResources/StandardMacros.IsValid` _skeletalmesh
        (:`Is Valid`
          (`SkinnedMeshComponent.SetSkinnedAssetAndUpdate` (`self.Mesh_Skeletal`) _skeletalmesh true))))))