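; BP_Computer is an interactable computer actor that opens and closes a full UI screen for the first local player.
; Interact toggles on IsBeingUsed, creating or removing a WBP_ComputerScreen widget while switching mouse cursor visibility and input mode between UI-only and game-only.
; It returns a fixed enum value to the caller.
; AttachToPhysicsHandle is a stub returning zero, and the event graph is empty.
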(fn `AttachToPhysicsHandle`
  (returns (`Distance From Camera` :type "Float (double-precision)"))
  (return 0.0))

(fn `Interact`
  (returns (`Interaction Type` :type "/Game/Blueprints/Enums/E_InteractionType Enum"))
  (bind _returnvalue (`GameplayStatics.GetPlayerController` 0))
  (bind _returnvalue_2 (`GameplayStatics.GetPlayerController` 0))
  (if (`self.isBeingUsed?`)
    (`Widget.RemoveFromParent` (`self.WidgetRef`))
    (set `self.WidgetRef` null)
    (set `self.isBeingUsed?` false)
    (set `PlayerController.bShowMouseCursor` false _returnvalue)
    (`WidgetBlueprintLibrary.SetInputMode_GameOnly` _returnvalue)
    (else
      (bind _returnvalue_3 (`|CreateWidget` "/Game/Blueprints/Widgets/WBP_ComputerScreen.WBP_ComputerScreen_C" _returnvalue_2))
      (set `self.WidgetRef` _returnvalue_3)
      (`UserWidget.AddToViewport` _returnvalue_3 0)
      (set `self.isBeingUsed?` true)
      (set `PlayerController.bShowMouseCursor` true _returnvalue_2)
      (`WidgetBlueprintLibrary.SetInputMode_UIOnlyEx` _returnvalue_2 (`self.WidgetRef`))))
  (return "NewEnumerator2"))

(fn `UserConstructionScript`)