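; BP_PATH_Details holds the road and parking spline paths for AI cars and acts as their spawner.
; Two seconds after BeginPlay it spawns one BP_AI_CAR at the start of a randomly picked straight-road spline, passing it a path and itself.
; Helper functions find the first free parking spot, book it and return its path, and supply reverse and leaving paths.
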(event `SpawnCar`
  (bind _straightroadpaths (break `/Game/VehicleAdvBP/Blueprints/Structs/Path_Properties` (`self.PathProperties`)))
  (bind _path (`/Game/VehicleAdvBP/Blueprints/CAR_BP/Path.Path` (`|GetArrayItem` _straightroadpaths (`KismetMathLibrary.RandomInteger` (- (`KismetArrayLibrary.Array_Length` _straightroadpaths) 1)))))
  (bind _returnvalue (`AIBlueprintHelperLibrary.SpawnAIFromClass` "/Game/VehicleAdvBP/Blueprints/CAR_BP/BP_AI_CAR.BP_AI_CAR_C" null (`SplineComponent.GetLocationAtSplinePoint` _path 0 "World") (struct) true null))
  (message `/Game/VehicleAdvBP/Blueprints/BPI_AI_VEHICLES.SetPath` _returnvalue _path self))

(event `self.ReceiveBeginPlay`
  (`KismetSystemLibrary.K2_SetTimerDelegate` (delegate `SpawnCar`) 2.0))

(fn `BookParkingSpot`
  (params (ParkingIndex :type Integer))
  (returns (Spline :type "SplineComponent Object Reference"))
  (bind (_pathproperties_straightroadpaths _pathproperties_leavingpaths _pathproperties_parkingspots) (break `/Game/VehicleAdvBP/Blueprints/Structs/Path_Properties` (`self.PathProperties`)))
  (bind _structout (setmembers `/Game/VehicleAdvBP/Blueprints/Structs/Parking_Properties` :`StructRef` (`|GetArrayItem` _pathproperties_parkingspots ParkingIndex) :`IsBooked` true))
  (return (`/Game/VehicleAdvBP/Blueprints/CAR_BP/Path.Path` (break `/Game/VehicleAdvBP/Blueprints/Structs/Parking_Properties` _structout))))

(fn `GetParkingSpot`
  (returns (IsSpotAvaliable :type Boolean) (IndexForParking :type Integer))
  (locals (NewLocalVar_0 :type "/Game/VehicleAdvBP/Blueprints/CAR_BP/Path Object Reference") (ParkingIndex :type Integer) (Isbooked :type Boolean))
  (bind (_pathproperties_straightroadpaths _pathproperties_leavingpaths _pathproperties_parkingspots) (break `/Game/VehicleAdvBP/Blueprints/Structs/Path_Properties` (`self.PathProperties`)))
  (for (_array_element _array_index) _pathproperties_parkingspots
    (set `local.Isbooked` (`.IsBooked_5_AA00407F4AE064AF9B23659ADEAD1F49` (break `/Game/VehicleAdvBP/Blueprints/Structs/Parking_Properties` _array_element)))
    (set `local.ParkingIndex` _array_index)
    (if (not (`.IsBooked_5_AA00407F4AE064AF9B23659ADEAD1F49` (break `/Game/VehicleAdvBP/Blueprints/Structs/Parking_Properties` _array_element)))
      (break)))
  (if (`local.Isbooked`)
    (return false 0)
    (else
      (return true (`local.ParkingIndex`)))))

(fn `GetRetunPath`
  (returns (`Return Path` :type "SplineComponent Object Reference"))
  (return (`/Game/VehicleAdvBP/Blueprints/CAR_BP/Path.Path` (`|GetArrayItem` (`.LeavingPaths_12_5DA603BB43C2C60FB8E00B8EABB5F38E` (break `/Game/VehicleAdvBP/Blueprints/Structs/Path_Properties` (`self.PathProperties`)))))))

(fn `GetReversePath`
  (params (PathIndex :type Integer))
  (returns (ReversePath :type "SplineComponent Object Reference"))
  (bind (_pathproperties_straightroadpaths _pathproperties_leavingpaths _pathproperties_parkingspots) (break `/Game/VehicleAdvBP/Blueprints/Structs/Path_Properties` (`self.PathProperties`)))
  (bind (_output_path _output_reversepath) (break `/Game/VehicleAdvBP/Blueprints/Structs/Parking_Properties` (`|GetArrayItem` _pathproperties_parkingspots PathIndex)))
  (return (`/Game/VehicleAdvBP/Blueprints/CAR_BP/Path.Path` _output_reversepath)))

(fn `UserConstructionScript`)