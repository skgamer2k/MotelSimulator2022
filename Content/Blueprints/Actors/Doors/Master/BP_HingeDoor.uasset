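; BP_HingeDoor is a master hinged door actor that swings open or closed when its InteractDoor event is called.
; InteractDoor toggles CurrentState between two values, playing or reversing the OpenClose timeline.
; The timeline's alpha lerps the DoorMesh relative yaw so the door rotates a quarter turn in a single fixed direction.
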(event `self.InteractDoor`
  (switch `int` (`self.CurrentState`)
    (:`0`
      (set `self.CurrentState` 1)
      (bind (_direction _open_close) (`Timeline|Open/Close` :!label _label)
        (:`Update`
          (`SceneComponent.K2_SetRelativeRotation` (`self.DoorMesh`) (`KismetMathLibrary.MakeRotator` 0.0 0.0 (`KismetMathLibrary.Lerp` 0.0 -90.0 _open_close)) false false))))
    (:`1`
      (set `self.CurrentState` 0)
      (goto _label :!via `Reverse`))))

(fn `UserConstructionScript`
  (`parent.UserConstructionScript`))