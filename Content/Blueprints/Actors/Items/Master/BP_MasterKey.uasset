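; BP_MasterKey is a key item actor, apparently the master class for keys, that the player can interact with and equip.
; It always reports itself as interactable, and Interact passes the key to player character 0 through an EquipKey message, then returns a fixed enum result.
; AttachToPhysicsHandle returns zero, and BeginPlay stores the starting location, which no graph here reads.
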(event `self.ReceiveBeginPlay`
  (set `self.InitialLocation` (`self.K2_GetActorLocation`)))

(fn `AttachToPhysicsHandle`
  (returns (`Distance From Camera` :type "Float (double-precision)"))
  (return 0.0))

(fn `CanBeInteracted?`
  (returns (`CanInteract?` :type Boolean))
  (return true))

(fn `Interact`
  (returns (`Interaction Type` :type "/Game/Blueprints/Enums/E_InteractionType Enum"))
  (message `/Game/Blueprints/Interfaces/BPI_Player.EquipKey` (`GameplayStatics.GetPlayerCharacter` 0) self)
  (return "NewEnumerator5"))

(fn `UserConstructionScript`)