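; BP_NPC_Male1 is a motel guest NPC that waits at a counter, receives a room key and walks into its room.
; Its detection volume flags the AnimBP when the player is near, for look-at, and being on the counter makes it interactable.
; On key receipt it finds the matching room via BP_MotelRoomsManager, feeds door locations to the BehaviorComponent and Blackboard, then switches behaviors.
; Further events open the door, change behavior to go inside, and despawn it.
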(event `self.ReceiveBeginPlay`
  ;[1 1 1] Saving AnimBP
  (bind _asabp_npc_male (cast `/Game/Blueprints/AICharacters/ABP_NPC_Male` (`SkeletalMeshComponent.GetAnimInstance` (`self.Mesh`))))
  (set `self.AnimBPReference` _asabp_npc_male))

(event `self.PlayerDetection.OnComponentBeginOverlap`
  (params (OverlappedComponent :type "PrimitiveComponent Object Reference") (OtherActor :type "Actor Object Reference") (OtherComp :type "PrimitiveComponent Object Reference") (OtherBodyIndex :type Integer) (bFromSweep :type Boolean) (SweepResult :type "HitResult Structure (by ref)"))
  ;[1 1 1] Logic for Look at PLayer
  (if (== OtherActor (`GameplayStatics.GetPlayerCharacter` 0))
    (set `/Game/Blueprints/AICharacters/ABP_NPC_Male.IsPlayerNear?` true (`self.AnimBPReference`))))

(event `self.PlayerDetection.OnComponentEndOverlap`
  (params (OverlappedComponent :type "PrimitiveComponent Object Reference") (OtherActor :type "Actor Object Reference") (OtherComp :type "PrimitiveComponent Object Reference") (OtherBodyIndex :type Integer))
  ;[1 1 1] Logic for Look at PLayer
  (if (== OtherActor (`GameplayStatics.GetPlayerCharacter` 0))
    (set `/Game/Blueprints/AICharacters/ABP_NPC_Male.IsPlayerNear?` false (`self.AnimBPReference`))))

(event `/Game/Blueprints/Interfaces/BPI_AI_NPC.UpdateIsOnCounter`
  (params (`isOnCounter?` :type Boolean))
  (set `self.Can Interact?` `isOnCounter?`))

(event `/Game/Blueprints/Interfaces/BPI_AI_NPC.UpdateKeyAcquired`
  (params (Key :type "/Game/Blueprints/Actors/Items/Master/BP_MasterKey Object Reference"))
  (bind _behaviorcomponent (`self.BehaviorComponent`))
  (set `self.Key` Key)
  (`/Engine/EditorBlueprintResources/StandardMacros.IsValid` Key
    (:`Is Valid`
      (bind _outactors (`GameplayStatics.GetAllActorsOfClass` "/Game/Blueprints/Motel2/Manager/BP_MotelRoomsManager.BP_MotelRoomsManager_C"))
      (for _array_element (`/Game/Blueprints/Motel2/Manager/BP_MotelRoomsManager.Rooms` (`|GetArrayItem` _outactors))
        (if (== (`.RoomID_4_A57BAEA842382131F4ED0B9CE19E926C` (break `/Game/Blueprints/Structs/MotelManagement/S_MotelRoomManager` _array_element)) (`/Game/Blueprints/Actors/Items/Master/BP_MasterKey.KeyID` (`self.Key`)))
          (break)))
      (bind (_isbooked_ _roomid _roomdooroutsidelocation _roomdoorinsidelocation _roomdooractor) (break `/Game/Blueprints/Structs/MotelManagement/S_MotelRoomManager` _array_element))
      (set `self.Room Door Actor` _roomdooractor)
      (set `/Game/AIBehaviorToolkit/Blueprints/BP_BehaviorComponent.GotoRoomTarget` _roomdooroutsidelocation _behaviorcomponent)
      (set `/Game/AIBehaviorToolkit/Blueprints/BP_BehaviorComponent.GoInsideRoomTarget` _roomdoorinsidelocation _behaviorcomponent)
      (set `self.Can Interact?` false)
      (`/Game/AIBehaviorToolkit/Blueprints/BP_BehaviorComponent.ChangeBehavior` (`self.BehaviorComponent`) "NewEnumerator14" false)
      (`BlackboardComponent.SetValueAsObject` (`AIBlueprintHelperLibrary.GetBlackboard` (`self.GetController`)) "Door" (`self.Room Door Actor`))
      (`self.K2_DestroyActor` (`self.Key`))
      (message `/Game/Blueprints/Interfaces/BPI_Player.UnequipKey` (`GameplayStatics.GetPlayerCharacter` 0)))))

(event `/Game/Blueprints/Interfaces/BPI_AI_NPC.InteractWithDoor`
  (message `/Game/Blueprints/Interfaces/BPI_Interactable.Interact` (`self.Room Door Actor`)))

(event `/Game/Blueprints/Interfaces/BPI_AI_NPC.Despawn`
  (`/Game/AIBehaviorToolkit/Blueprints/Interfaces/BPI_Commands.CommandStopBrain`)
  (`self.K2_DestroyActor`))

(event `/Game/Blueprints/Interfaces/BPI_AI_NPC.GoInsideRoom`
  (`/Game/AIBehaviorToolkit/Blueprints/BP_BehaviorComponent.ChangeBehavior` (`self.BehaviorComponent`) "NewEnumerator17" false))

(fn `AttachToPhysicsHandle`
  (returns (`Distance From Camera` :type "Float (double-precision)"))
  (return 0.0))

(fn `CanBeInteracted?`
  (returns (`CanInteract?` :type Boolean))
  (return (`self.Can Interact?`)))

(fn `GetKeyInfo`
  (returns (Key :type "/Game/Blueprints/Actors/Items/Master/BP_MasterKey Object Reference"))
  (return null))

(fn `Interact`
  (returns (`Interaction Type` :type "/Game/Blueprints/Enums/E_InteractionType Enum"))
  (return "NewEnumerator6"))

(fn `UserConstructionScript`
  (`parent.UserConstructionScript`))